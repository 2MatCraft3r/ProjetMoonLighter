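; Player character Blueprint that handles movement, a dodge roll, and light and heavy attacks.
; Enhanced Input moves it along fixed world axes when CanMove is set and snaps the mesh rotation from the input direction.
; Space, left and right mouse are raw key events playing montages, with the roll requiring ground and playing faster at higher speed.
; Boolean flags and Delays gate repeats, with both attacks sharing a lock and the heavy one cooling down longer.
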(event `self.ReceiveBeginPlay`
  (bind _asplayer_controller (cast `PlayerController` (`self.GetController`)))
  (`EnhancedInputSubsystemInterface.AddMappingContext` (pcsubsystem `EnhancedInputLocalPlayerSubsystem` _asplayer_controller) "/Game/Inputs/IMC_Player.IMC_Player" 0 (struct))
  (set `self.RotationInitial` (struct :`Yaw` -90.0)))

(event `self.ReceiveTick`
  (params (DeltaSeconds :type "Float (single-precision)")))

(event `EnhancedInput|/Game/Inputs/Actions/IA_Move`
  (params (ActionValue :type "Vector2D Structure") (ElapsedSeconds :type "Float (double-precision)") (TriggeredSeconds :type "Float (double-precision)") (InputAction :type "InputAction Object Reference" :default "/Game/Inputs/Actions/IA_Move.IA_Move"))
  (:`Triggered`
    (if (`self.CanMove`)
      (`self.AddMovementInput` (-1.0 0.0 0.0) ActionValue_X)
      (`self.AddMovementInput` (0.0 -1.0 0.0) ActionValue_Y)
      (if (== ActionValue_X -1.0)
        (`SceneComponent.K2_SetWorldRotation` (`self.Mesh`) (`self.RotationInitial`) false false)
        (elif (== ActionValue_X 1.0)
          (bind _output_get (set `self.NouvelleValeur` (`KismetMathLibrary.Conv_VectorToRotator` (+ (`self.RotationInitial`) (0.0 180.0 0.0)))))
          (`SceneComponent.K2_SetWorldRotation` (`self.Mesh`) _output_get false false)
          (elif (>= ActionValue_Y 1.0)
            (bind _output_get_2 (set `self.NouvelleValeur` (`KismetMathLibrary.Conv_VectorToRotator` (+ (`self.RotationInitial`) (-90.0 0.0 0.0)))))
            (`SceneComponent.K2_SetWorldRotation` (`self.Mesh`) _output_get_2 false false)
            (elif (>= ActionValue_Y -1.0)
              (bind _output_get_3 (set `self.NouvelleValeur` (`KismetMathLibrary.Conv_VectorToRotator` (+ (`self.RotationInitial`) (90.0 0.0 0.0)))))
              (`SceneComponent.K2_SetWorldRotation` (`self.Mesh`) _output_get_3 false false))))))))

(event `Key|SpaceBar`
  (params (Key :type "Key Structure"))
  (bind _charactermovement (`self.CharacterMovement`))
  (:`Pressed`
    (if (`self.Roll`)
      (set `self.Roll` false)
      (if (not (`NavMovementComponent.IsFalling` _charactermovement))
        (`/Engine/EditorBlueprintResources/StandardMacros.DoOnce` false :!label _label
          (:`Completed`
            (if (> (`KismetMathLibrary.VSize` (`MovementComponent.Velocity` _charactermovement)) 300.0)
              (set `self.Float1` 1.5)
              (else
                (set `self.Float1` 1.2)))
            (`|PlayMontage` (`self.Mesh`) "/Game/Sword_Animations/Animations/Sequence1/07_Roll/02_Roll_Combat/M_Roll.M_Roll" (`self.Float1`)
              (:`then`
                (goto _label :!via `Reset`))
              (:`OnCompleted`
                (`KismetSystemLibrary.Delay` 0.2)
                (set `self.Roll` true)))))))))

(event `Key|LeftMouseButton`
  (params (Key :type "Key Structure"))
  (:`Pressed`
    (if (and (`self.CanAttackDouce`) (`self.Attack`))
      (set `self.CanAttackDouce` false)
      (set `self.Attack` false)
      (`|PlayMontage` (`self.Mesh`) "/Game/Sword_Animations/Animations/Sequence1/02_Attack/04_Combo_Attack_04/M_AttackBas.M_AttackBas"
        (:`then`
          (`KismetSystemLibrary.Delay` 1.5)
          (set `self.CanAttackDouce` true)
          (set `self.Attack` true))))))

(event `Key|RightMouseButton`
  (params (Key :type "Key Structure"))
  (:`Pressed`
    (if (and (`self.Attack`) (`self.Can AttackForte`))
      (set `self.Attack` false)
      (set `self.Can AttackForte` false)
      (`|PlayMontage` (`self.Mesh`) "/Game/Sword_Animations/Animations/Sequence1/02_Attack/12_Run_Attact/M_AttackLourde.M_AttackLourde"
        (:`then`
          (`KismetSystemLibrary.Delay` 1.5)
          (set `self.Attack` true)
          (`KismetSystemLibrary.Delay` 1.0)
          (set `self.Can AttackForte` true))))))

(fn `UserConstructionScript`)